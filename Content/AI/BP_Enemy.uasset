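; BP_Enemy is an enemy actor that periodically drops a BP_CollectedEctoplasm at its location and can be frozen or destroyed.
; BeginPlay rolls a random spawn delay and starts a looping timer; later rerolls update the variable but never reset that timer.
; FreezeOnServer forwards to FreezeOnClient, which zeroes custom time dilation until a timer restores it.
; Event names indicate a server/client split, with DeathOnServer destroying the actor.
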(event Custom|Spawn%20Ecto%20On%20Server
  (Game|SpawnActorfromClass "/Game/BP_CollectedEctoplasm.BP_CollectedEctoplasm_C" (Transformation|GetActorTransform) "AdjustIfPossibleButAlwaysSpawn" "MultiplyWithRoot" 0 0)
  (CallFunction|NewTimeonServer))

(event Custom|New%20Time%20On%20Server
  (Variables|Default|SetTime%20to%20spawn (Math|Random|RandomFloatinRange 1e+01 6e+01)))

(event Custom|Death%20On%20Server
  (Actor|DestroyActor))

(event Custom|Freeze%20On%20Server
  (params (Time%20To%20Freeze :type Float%20%28single-precision%29))
  (CallFunction|FreezeonClient Time%20To%20Freeze))

(event Custom|Unfreeze
  (Variables|Default|SetCustomTimeDilation 1.0))

(event Custom|Freeze%20On%20Client
  (params (Time%20To%20Freeze :type Float%20%28single-precision%29))
  (Variables|Default|SetCustomTimeDilation 0.0)
  (Utilities|Time|SetTimerbyEvent (delegate Custom|Unfreeze) Time%20To%20Freeze))

(event EventBeginPlay
  (CallFunction|NewTimeonServer)
  (Utilities|Time|SetTimerbyEvent (delegate Custom|Spawn%20Ecto%20On%20Server) (Variables|Default|GetTime%20to%20spawn) true))

(fn ConstructionScript)