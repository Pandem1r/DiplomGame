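; Multiplayer player character with Enhanced Input movement, crouch, run, health, and ectoplasm pickup and dropping.
; A camera sphere trace on Tick finds interactable actors; pickups can destroy them or raise the GameState ectoplasm total and check for a win.
; Actions route through OnServer/OnClient event pairs, while RepNotifies broadcast health and count changes.
; Death ragdolls the body, scatters carried ectoplasm, informs the GameMode, and enables cycling through players to spectate.
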(event Custom|Pickup%20On%20Server
  (params (InputObject :type Object%20Object%20Reference))
  (Utilities|IsValid InputObject
    (:Is%20Valid
      (CallFunction|PickuponClient InputObject))))

(event Custom|Pickup%20on%20Client
  (params (Target :type Object%20Object%20Reference))
  (bind (_targettodestroy _destroyed _incrementectoplasm) (Class|IInteraction|Pickup(Message) Target self))
  (if _destroyed
    (CallFunction|DestroyonServer _targettodestroy)
    (elif _incrementectoplasm
      (CallFunction|IncrementEctoplasmonServer))))

(event Custom|Previous%20Player%20On%20Client
  (bind _gamestate (Variables|Default|GetGameState))
  (bind _playerarray (Variables|/Script/Engine.GameStateBase|GetPlayerArray _gamestate))
  (if (== (- (Variables|Default|GetCurrent%20Player) 1) -1)
    (Variables|Default|SetCurrent%20Player (Utilities|Array|LastIndex _playerarray))
    (else
      (Variables|Default|SetCurrent%20Player (- (Variables|Default|GetCurrent%20Player) 1))))
  (Game|Player|SetViewTargetwithBlend (Game|GetPlayerController 0) (Utilities|Array|Get(acopy) _playerarray (Variables|Default|GetCurrent%20Player)) 0.0 "VTBlend_Linear" 0.0 false))

(event Custom|Game%20Over%20Screen%20on%20Client
  (bind _returnvalue (UserInterface|CreateWidget "/Game/UI/WB_GameOver.WB_GameOver_C" (Game|GetPlayerController 0)))
  (UserInterface|Viewport|AddtoViewport _returnvalue 0))

(event Custom|Next%20Player%20On%20Server
  (CallFunction|NextPlayeronClient))

(event Custom|Death%20On%20Server
  (params (WhoDead :type BP%20Character%20Object%20Reference))
  (Variables|BP_Character_C|SetIsDead WhoDead true)
  (CallFunction|DeathonOwn)
  (CallFunction|DeathonClient))

(event Custom|Death%20On%20Client
  (bind _mesh (Variables|Character|GetMesh))
  (Pawn|Components|CharacterMovement|DisableMovement (Variables|Character|GetCharacterMovement))
  (Physics|SetSimulatePhysics _mesh true)
  (Collision|SetCollisionEnabled _mesh "PhysicsOnly")
  (Collision|SetCollisionEnabled (Variables|Collision|GetCapsuleComponent) "NoCollision")
  (for _index (range 0 (- (Variables|Ectoplasm|GetCurrentCount) 1))
    (CallFunction|DroponServer (Math|Transform|MakeTransform (+ (Transformation|GetActorLocation) (Math|Vector|MakeVector (Math|Random|RandomFloatinRange 0.0 1e+02) (Math|Random|RandomFloatinRange 0.0 1e+02) 5e+01))) "/Game/BP_CollectedEctoplasm.BP_CollectedEctoplasm_C")))

(event Custom|Previous%20Player%20on%20Server
  (CallFunction|PreviousPlayeronClient))

(event Custom|Death%20on%20Own
  (Input|SetIgnoreLookInput (Pawn|GetController) true)
  (Default|CallOnIsDeadChanged)
  (Utilities|IsValid (Variables|Default|GetGameState)
    (:Is%20Not%20Valid
      (bind _asbp_main_game_state (Utilities|Casting|CastToBP_MainGameState (Game|GetGameState)))
      (Variables|Default|SetGameState _asbp_main_game_state))))

(event Custom|Next%20Player%20On%20Client
  (bind _gamestate (Variables|Default|GetGameState))
  (bind _playerarray (Variables|/Script/Engine.GameStateBase|GetPlayerArray _gamestate))
  (if (== (Variables|Default|GetCurrent%20Player) (Utilities|Array|LastIndex _playerarray))
    (Variables|Default|SetCurrent%20Player 0)
    (else
      (Variables|Default|SetCurrent%20Player (+ (Variables|Default|GetCurrent%20Player) 1))))
  (Game|Player|SetViewTargetwithBlend (Game|GetPlayerController 0) (Utilities|Array|Get(acopy) _playerarray (Variables|Default|GetCurrent%20Player)) 0.0 "VTBlend_Linear" 0.0 false))

(event Custom|Increment%20Ectoplasm%20on%20Server
  (Utilities|IsValid (Variables|Default|GetGameState)
    (:Is%20Valid
      _)
    (:Is%20Not%20Valid
      (bind _asbp_main_game_state (Utilities|Casting|CastToBP_MainGameState (Game|GetGameState)))
      (Variables|Default|SetGameState _asbp_main_game_state)))
  (Variables|/Game/BP_MainGameState.BP_MainGameState_C|SetEctoplasmCurrent (Variables|Default|GetGameState) (+ (Variables|/Game/BP_MainGameState.BP_MainGameState_C|GetEctoplasmCurrent (Variables|Default|GetGameState)) 1))
  (Default|CheckWin (Variables|Default|GetGameState)))

(event Custom|Run%20On%20Client
  (params (IsRunning :type Boolean))
  (bind _charactermovement (Variables|Character|GetCharacterMovement))
  ;[1 1 1] Бег + репликация
  (if IsRunning
    (Variables|/Script/Engine.CharacterMovementComponent|SetMaxWalkSpeed _charactermovement (Variables|Movement|GetRunningSpeed))
    (else
      (Variables|/Script/Engine.CharacterMovementComponent|SetMaxWalkSpeed _charactermovement (Variables|Movement|GetWalkingSpeed)))))

(event Custom|Crouching%20On%20Server
  (params (IsCrouching :type Boolean))
  ;[1 1 1] Красться + репликация
  (CallFunction|CrouchingonClient IsCrouching))

(event Custom|Crouching%20On%20Client
  (params (IsCrouching :type Boolean))
  (bind _charactermovement (Variables|Character|GetCharacterMovement))
  ;[1 1 1] Красться + репликация
  (if IsCrouching
    (Variables|/Script/Engine.CharacterMovementComponent|SetMaxWalkSpeed _charactermovement (Variables|Movement|GetCrouchingSpeed))
    (else
      (Variables|/Script/Engine.CharacterMovementComponent|SetMaxWalkSpeed _charactermovement (Variables|Movement|GetWalkingSpeed)))))

(event Custom|Drop%20On%20Server
  (params (SpawnTransform :type Transform) (Class :type Actor%20Class%20Reference))
  (Game|SpawnActorfromClass Class SpawnTransform "AlwaysSpawn" "MultiplyWithRoot" 0 0))

(event Custom|Run%20On%20Server
  (params (IsRunning :type Boolean))
  ;[1 1 1] Бег + репликация
  (CallFunction|RunonClient IsRunning))

(event Custom|Destroy%20On%20Server
  (params (Target :type Actor%20Object%20Reference))
  (Utilities|IsValid Target
    (:Is%20Valid
      (Actor|DestroyActor Target))))

(event Custom|Damage%20on%20Server
  (Game|Damage|ApplyDamage self 2e+01 0 0))

(event Input|EnhancedActionEvents|EnhancedInputActionIA_Interact
  (params (ActionValue :type Boolean) (ElapsedSeconds :type Float%20%28double-precision%29) (TriggeredSeconds :type Float%20%28double-precision%29) (InputAction :type Input%20Action%20Object%20Reference :default "/Game/Input/IA_Interact.IA_Interact"))
  (:Started
    (CallFunction|PickuponServer (Variables|Default|GetLookAtActor))))

(event Input|EnhancedActionEvents|EnhancedInputActionIA_Look
  (params (ActionValue :type Vector%202D%20Structure) (ElapsedSeconds :type Float%20%28double-precision%29) (TriggeredSeconds :type Float%20%28double-precision%29) (InputAction :type Input%20Action%20Object%20Reference :default "/Game/Input/IA_Look.IA_Look"))
  ;[1 1 1] Вращение камеры
  (Pawn|Input|AddControllerYawInput (.x ActionValue))
  (Pawn|Input|AddControllerPitchInput (* (.y ActionValue) -1.0)))

(event Input|EnhancedActionEvents|EnhancedInputActionIA_Move
  (params (ActionValue :type Vector%202D%20Structure) (ElapsedSeconds :type Float%20%28double-precision%29) (TriggeredSeconds :type Float%20%28double-precision%29) (InputAction :type Input%20Action%20Object%20Reference :default "/Game/Input/IA_Move.IA_Move"))
  (bind _returnvalue (Pawn|GetControlRotation :!class /Script/Engine.Pawn))
  ;[1 1 1] Движение
  (Pawn|Input|AddMovementInput (Math|Vector|GetRightVector (Math|Rotator|MakeRotator (.roll _returnvalue) 0.0 (.yaw _returnvalue))) (.x ActionValue) false)
  (Pawn|Input|AddMovementInput (Math|Vector|GetForwardVector (Math|Rotator|MakeRotator 0.0 0.0 (.yaw (Pawn|GetControlRotation :!class /Script/Engine.Pawn)))) (.y ActionValue) false))

(event Input|EnhancedActionEvents|EnhancedInputActionIA_Crouch
  (params (ActionValue :type Boolean) (ElapsedSeconds :type Float%20%28double-precision%29) (TriggeredSeconds :type Float%20%28double-precision%29) (InputAction :type Input%20Action%20Object%20Reference :default "/Game/Input/IA_Crouch.IA_Crouch"))
  ;[1 1 1] Красться + репликация
  (:Started
    (CallFunction|CrouchingonServer ActionValue))
  (:Completed
    (CallFunction|CrouchingonServer ActionValue)))

(event Input|EnhancedActionEvents|EnhancedInputActionIA_Jump
  (params (ActionValue :type Boolean) (ElapsedSeconds :type Float%20%28double-precision%29) (TriggeredSeconds :type Float%20%28double-precision%29) (InputAction :type Input%20Action%20Object%20Reference :default "/Game/Input/IA_Jump.IA_Jump"))
  ;[1 1 1] Прыжок
  (:Started
    (Character|Jump))
  (:Completed
    (Character|StopJumping)))

(event Input|EnhancedActionEvents|EnhancedInputActionIA_Run
  (params (ActionValue :type Boolean) (ElapsedSeconds :type Float%20%28double-precision%29) (TriggeredSeconds :type Float%20%28double-precision%29) (InputAction :type Input%20Action%20Object%20Reference :default "/Game/Input/IA_Run.IA_Run"))
  ;[1 1 1] Бег + репликация
  (:Started
    (CallFunction|RunonServer ActionValue))
  (:Completed
    (CallFunction|RunonServer ActionValue)))

(event Input|EnhancedActionEvents|EnhancedInputActionIA_UseItem
  (params (ActionValue :type Boolean) (ElapsedSeconds :type Float%20%28double-precision%29) (TriggeredSeconds :type Float%20%28double-precision%29) (InputAction :type Input%20Action%20Object%20Reference :default "/Game/Input/IA_UseItem.IA_UseItem"))
  (:Started
    (CallFunction|DamageonServer)))

(event Input|EnhancedActionEvents|EnhancedInputActionIA_Drop
  (params (ActionValue :type Boolean) (ElapsedSeconds :type Float%20%28double-precision%29) (TriggeredSeconds :type Float%20%28double-precision%29) (InputAction :type Input%20Action%20Object%20Reference :default "/Game/Input/IA_Drop.IA_Drop"))
  (:Started
    (if (> (Variables|Ectoplasm|GetCurrentCount) 0)
      (CallFunction|DroponServer (Math|Transform|MakeTransform (+ (Transformation|GetActorLocation) (* (Math|Vector|GetForwardVector (Transformation|GetActorRotation)) 1e+02))) "/Game/BP_CollectedEctoplasm.BP_CollectedEctoplasm_C")
      (Variables|Ectoplasm|SetCurrentCount (- (Variables|Ectoplasm|GetCurrentCount) 1)))))

(event Input|EnhancedActionEvents|EnhancedInputActionIA_SpectateNext
  (params (ActionValue :type Boolean) (ElapsedSeconds :type Float%20%28double-precision%29) (TriggeredSeconds :type Float%20%28double-precision%29) (InputAction :type Input%20Action%20Object%20Reference :default "/Game/Input/IA_SpectateNext.IA_SpectateNext"))
  (:Started
    (if (Variables|Default|GetIsDead)
      (CallFunction|NextPlayeronServer))))

(event Input|EnhancedActionEvents|EnhancedInputActionIA_SpectatePrevious
  (params (ActionValue :type Boolean) (ElapsedSeconds :type Float%20%28double-precision%29) (TriggeredSeconds :type Float%20%28double-precision%29) (InputAction :type Input%20Action%20Object%20Reference :default "/Game/Input/IA_SpectatePrevious.IA_SpectatePrevious"))
  (:Started
    (if (Variables|Default|GetIsDead)
      (CallFunction|PreviousPlayeronServer))))

(event EventBeginPlay
  ;[1 1 1] Подключение Input Mapping Context
  (bind _asplayer_controller (Utilities|Casting|CastToPlayerController (Pawn|GetController)))
  (Utilities|IsValid (PlayerController|LocalPlayerSubsystems|GetEnhancedInputLocalPlayerSubsystem _asplayer_controller)
    (:Is%20Valid
      (Input|AddMappingContext (PlayerController|LocalPlayerSubsystems|GetEnhancedInputLocalPlayerSubsystem _asplayer_controller) "/Game/Input/IMC_Character.IMC_Character" 0 "(bIgnoreAllPressedKeysUntilRelease=True,bForceImmediately=False,bNotifyUserSettings=False)"))))

(event EventTick
  (params (DeltaSeconds :type Float%20%28single-precision%29))
  (bind _returnvalue (Game|GetPlayerCameraManager 0))
  (bind _returnvalue_2 (Transformation|GetActorLocation _returnvalue))
  (bind (_outhit _returnvalue_3) (Collision|SphereTraceByChannel _returnvalue_2 (+ _returnvalue_2 (* (Transformation|GetActorForwardVector _returnvalue) (Variables|Ectoplasm|GetInteractionRange))) 1e+01 "TraceTypeQuery1" false 0 "None" true "(R=1.000000,G=0.000000,B=0.000000,A=1.000000)" "(R=0.000000,G=1.000000,B=0.000000,A=1.000000)" 3.0))
  (if _returnvalue_3
    (if (!= (.HitActor (Collision|BreakHitResult _outhit)) (Variables|Default|GetLookAtActor))
      (bind _output_get (Variables|Default|SetLookAtActor (.HitActor (Collision|BreakHitResult _outhit))))
      (Default|CallOnInteractChanged (Utilities|DoesObjectImplementInterface _output_get "/Game/IInteraction.IInteraction_C")))
    (else
      (Variables|Default|SetLookAtActor 0)
      (Default|CallOnInteractChanged false))))

(event Game|Damage|EventAnyDamage
  (params (Damage :type Float%20%28single-precision%29) (DamageType :type Damage%20Type%20Object%20Reference) (InstigatedBy :type Controller%20Object%20Reference) (DamageCauser :type Actor%20Object%20Reference))
  (if (not (Variables|Default|GetIsDead))
    (bind _output_get (Variables|Default|SetHealth (- (Variables|Default|GetHealth) Damage)))
    (if (<= _output_get 0.0)
      (CallFunction|DeathonServer self)
      (bind _asbp_main_game_mode (Utilities|Casting|CastToBP_MainGameMode (Game|GetGameMode)))
      (Default|DecreasePlayersAlive _asbp_main_game_mode))))

(event EventDestroyed
  (bind _asbp_main_game_mode (Utilities|Casting|CastToBP_MainGameMode (Game|GetGameMode)))
  (Default|DecreasePlayersAlive _asbp_main_game_mode))

(fn ConstructionScript)

(fn OnRepCurrentCount
  (Default|CallOnCountChanged (Variables|Ectoplasm|GetCurrentCount)))

(fn OnRepHealth
  (Default|CallOnHealthChanged (Variables|Default|GetHealth)))