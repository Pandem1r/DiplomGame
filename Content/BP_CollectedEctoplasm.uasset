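; BP_CollectedEctoplasm is an ectoplasm pickup that characters collect, and it destroys itself once a TimeToDestroy timer expires.
; Its mesh stops simulating physics on first hit and activates RotatingMovement to spin in place.
; Pickup increments the BP_Character's count up to MaxCount, printing debug text and returning whether the pickup should be destroyed, leaving that destruction to the caller.
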(event OnComponentHit(StaticMesh)
  (params (HitComponent :type Primitive%20Component%20Object%20Reference) (OtherActor :type Actor%20Object%20Reference) (OtherComp :type Primitive%20Component%20Object%20Reference) (NormalImpulse :type Vector :default "0, 0, 0") (Hit :type Hit%20Result%20Structure%20%28by%20ref%29))
  (Physics|SetSimulatePhysics (Variables|Default|GetStaticMesh) false)
  (Components|Activation|Activate (Variables|Default|GetRotatingMovement) false))

(event Custom|Destroy%20On%20Server
  (Actor|DestroyActor))

(event EventBeginPlay
  (Utilities|Time|SetTimerbyEvent (delegate Custom|Destroy%20On%20Server) (Variables|Default|GetTime%20To%20Destroy)))

(fn ConstructionScript)

(fn Pickup
  (params (WhoPicked :type Actor%20Object%20Reference))
  (bind _asbp_character (Utilities|Casting|CastToBP_Character WhoPicked))
  (if (< (Variables|/Game/BP_Character.BP_Character_C|GetCurrentCount _asbp_character) (Variables|/Game/BP_Character.BP_Character_C|GetMaxCount _asbp_character))
    (bind _output_get (Variables|/Game/BP_Character.BP_Character_C|SetCurrentCount _asbp_character (+ (Variables|/Game/BP_Character.BP_Character_C|GetCurrentCount _asbp_character) 1)))
    (Development|PrintString (Utilities|String|ToString(Integer) _output_get))
    (return self true false)
    (else
      (Development|PrintString "Max Count!")
      (return 0 false false))))