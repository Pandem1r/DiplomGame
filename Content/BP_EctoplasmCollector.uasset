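; BP_EctoplasmCollector is a deposit point where a character hands over carried ectoplasm toward the game's win target.
; Pickup takes one unit from BP_Character's CurrentCount, prints the new count, and returns IncrementEctoplasm while the game state total is below EctoplasmToWin.
; The game state reference is cached on BeginPlay and refetched if invalid.
; Pickup never destroys the collector or increments the total itself.
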(event EventBeginPlay
  (bind _asbp_main_game_state (Utilities|Casting|CastToBP_MainGameState (Game|GetGameState)))
  (Variables|Default|SetGameState _asbp_main_game_state))

(fn ConstructionScript)

(fn Pickup
  (params (WhoPicked :type Actor%20Object%20Reference))
  (bind _asbp_character (Utilities|Casting|CastToBP_Character WhoPicked))
  (if (> (Variables|/Game/BP_Character.BP_Character_C|GetCurrentCount _asbp_character) 0)
    (Utilities|IsValid (Variables|Default|GetGameState)
      (:Is%20Valid
        _)
      (:Is%20Not%20Valid
        (bind _asbp_main_game_state (Utilities|Casting|CastToBP_MainGameState (Game|GetGameState)))
        (Variables|Default|SetGameState _asbp_main_game_state)))
    (if (< (Variables|/Game/BP_MainGameState.BP_MainGameState_C|GetEctoplasmCurrent (Variables|Default|GetGameState)) (Variables|/Game/BP_MainGameState.BP_MainGameState_C|GetEctoplasmToWin (Variables|Default|GetGameState)))
      (bind _output_get (Variables|/Game/BP_Character.BP_Character_C|SetCurrentCount _asbp_character (+ (Variables|/Game/BP_Character.BP_Character_C|GetCurrentCount _asbp_character) -1)))
      (Development|PrintString (Utilities|String|ToString(Integer) _output_get))
      (return 0 false true)
      (else
        _)))
  (return 0 false false))