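; BP_MainGameMode is a game mode that counts living players and announces a loss when none remain.
; PostLogin increments PlayersAlive, while DecreasePlayersAlive decrements it and runs CheckPlayersAlive, which calls Lose at zero or below.
; Win and Lose only print messages, and nothing in this Blueprint calls Win.
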(event Custom|Win
  (Development|PrintString "You're winner!"))

(event Custom|Check%20Players%20Alive
  (if (<= (Variables|Default|GetPlayersAlive) 0)
    (CallFunction|Lose)))

(event Custom|Decrease%20Players%20Alive
  (bind _result (Math|Integer|DecrementInt (Variables|Default|GetPlayersAlive))
    (:%20%20
      (Variables|Default|SetPlayersAlive _result)
      (CallFunction|CheckPlayersAlive))))

(event Custom|Lose
  (Development|PrintString "Loser!"))

(event EventPostLogin
  (params (NewPlayer :type Player%20Controller%20Object%20Reference))
  (bind _result (Math|Integer|IncrementInt (Variables|Default|GetPlayersAlive))
    (:%20%20
      (Variables|Default|SetPlayersAlive _result))))

(fn ConstructionScript)