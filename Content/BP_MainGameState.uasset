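; BP_MainGameState is the game state Blueprint that checks the ectoplasm win condition.
; The construction script caches a reference to BP_MainGameMode.
; CheckWin compares current ectoplasm to the amount needed and, once reached, calls Win on the game mode, re-fetching the reference if it is invalid.
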(event Custom|CheckWin
  (if (>= (Variables|Default|GetEctoplasmCurrent) (Variables|Default|GetEctoplasmToWin))
    (Utilities|IsValid (Variables|Default|GetGameMode)
      (:Is%20Valid
        _)
      (:Is%20Not%20Valid
        (bind _asbp_main_game_mode (Utilities|Casting|CastToBP_MainGameMode (Game|GetGameMode)))
        (Variables|Default|SetGameMode _asbp_main_game_mode)))
    (Default|Win (Variables|Default|GetGameMode))))

(fn ConstructionScript
  (bind _asbp_main_game_mode (Utilities|Casting|CastToBP_MainGameMode (Game|GetGameMode)))
  (Variables|Default|SetGameMode _asbp_main_game_mode))